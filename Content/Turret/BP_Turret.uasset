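; BP_Turret is a turret actor that shoots at the first-person player character when it sees them.
; PawnSensing's See Pawn event filters for BP_FirstPersonCharacter and instantly rotates the whole actor to face the player's location.
; After a short delay it spawns a BP_Bullet at the Arrow component's transform and plays an attenuated explosion sound at the turret.
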(event `self.PawnSensing.OnSeePawn`
  (params (Pawn :type "Pawn Object Reference"))
  (cast `/Game/FirstPerson/Blueprints/BP_FirstPersonCharacter` Pawn)
  (`self.K2_SetActorRotation` (`KismetMathLibrary.FindLookAtRotation` (`self.K2_GetActorLocation`) (`self.K2_GetActorLocation` Pawn)))
  (`KismetSystemLibrary.Delay` 1.0)
  (`|SpawnActorFromClass` "/Game/Turret/BP_Bullet.BP_Bullet_C" (`SceneComponent.K2_GetComponentToWorld` (`self.Arrow`)) "AlwaysSpawn" "MultiplyWithRoot" null null)
  (`GameplayStatics.PlaySoundAtLocation` "/Game/FPWeapon/Audio/explosion_dull.explosion_dull" (`self.K2_GetActorLocation`) (struct) 0.5 1.0 0.0 "/Game/FirstPerson/DefaultSoundAttenuation.DefaultSoundAttenuation" null null null))

(fn `UserConstructionScript`)